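; BP_Flower_Sprite is a 2D flipbook flower that starts as a static-type sprout and grows into a 3D flower.
; The construction script picks the sprout flipbook by FlowerType, and Tick yaws it toward the player camera as a billboard.
; Grow runs once, playing a per-type growth animation and delay, then replaces the actor with a small-scaled BP_Flower3D carrying FlowerType, Pot and SlotNum.
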(event Custom|Grow
  (bind _paperflipbook (Variables|Default|GetPaperFlipbook))
  (bind _flower_type (Variables|Default|GetFlower%20Type))
  (bind _returnvalue (- _flower_type 1))
  (if (not (Variables|Default|GetisGrow))
    (Variables|Default|SetisGrow true)
    (Sprite|SetFlipbook _paperflipbook (Utilities|Select :Index _returnvalue :Option%200 "/Game/Cait/Asset/2DSprite/Flower1_Flipbook.Flower1_Flipbook" :Option%201 "/Game/Cait/Asset/2DSprite/Flower2_Flipbook.Flower2_Flipbook" :Option%202 "/Game/Cait/Asset/2DSprite/Flower3_Flipbook.Flower3_Flipbook"))
    (Components|Timeline|SetPlayRate _paperflipbook (Utilities|Select :Index _returnvalue :Option%200 2.0 :Option%201 1.0 :Option%202 0.5))
    (Utilities|FlowControl|Delay (Utilities|Select :Index _returnvalue :Option%200 4.5 :Option%201 9.5 :Option%202 14.5))
    (Actor|DestroyActor)
    (Game|SpawnActorfromClass "/Game/Blueprint/Flower/BP_Flower3D.BP_Flower3D_C" (Math|Transform|MakeTransform (Transformation|GetActorLocation) "0, 0, 0" "0.050000,0.050000,0.050000") "Undefined" "OverrideRootScale" 0 (Variables|Default|GetFlower%20Type) (Variables|Default|GetPot) (Variables|Default|GetSlotNum) 0)))

(event EventBeginPlay)

(event Collision|EventActorBeginOverlap
  (params (OtherActor :type Actor%20Object%20Reference)))

(event EventTick
  (params (DeltaSeconds :type Float%20%28single-precision%29))
  (CallFunction|RotatetoCamera))

(fn ConstructionScript
  (Sprite|SetFlipbook (Variables|Default|GetPaperFlipbook) (Utilities|Select :Index (- (Variables|Default|GetFlower%20Type) 1) :Option%200 "/Game/Cait/Asset/2DSprite/Flower1_Tunas.Flower1_Tunas" :Option%201 "/Game/Cait/Asset/2DSprite/Flower2_Tunas.Flower2_Tunas" :Option%202 "/Game/Cait/Asset/2DSprite/Flower3_Tunas.Flower3_Tunas")))

(fn RotatetoCamera
  (Transformation|SetWorldRotation (Variables|Default|GetPaperFlipbook) (Math|Rotator|MakeRotator 0.0 0.0 (+ (.yaw (Math|Rotator|FindLookatRotation (Transformation|GetActorLocation) (Transformation|GetActorLocation (Game|GetPlayerCameraManager 0)))) 9e+01)) false false))