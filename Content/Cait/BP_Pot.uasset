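; BP_Pot is a planting pot with a fixed set of slots that turns seeds into flowers.
; When a BP_SeedA overlaps its Sphere, it spawns a BP_Flower_Sprite of that type at the first free slot's child component, then respawns and destroys the seed.
; A Slot map tracks occupancy, and DeactivateSlot frees an entry.
; GrowPlant calls Grow on flowers planted since its last call, then clears that list.
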(event OnComponentBeginOverlap(Sphere)
  (params (OverlappedComponent :type Primitive%20Component%20Object%20Reference) (OtherActor :type Actor%20Object%20Reference) (OtherComp :type Primitive%20Component%20Object%20Reference) (OtherBodyIndex :type Integer) (bFromSweep :type Boolean) (SweepResult :type Hit%20Result%20Structure%20%28by%20ref%29))
  (bind _slot (Variables|Default|GetSlot))
  (bind _asbp_seed_a (Utilities|Casting|CastToBP_SeedA OtherActor))
  (bind _keys (Utilities|Map|Keys _slot))
  (bind _array_element (Utilities|Array|ForEachLoopwithBreak _keys :!label _label)
    (:LoopBody
      (if (not (.Value (Utilities|Map|Find _slot _array_element)))
        (bind _returnvalue (Game|SpawnActorfromClass "/Game/Cait/BP_Flower_Sprite.BP_Flower_Sprite_C" (Math|Transform|MakeTransform (.location (Transformation|GetSocketTransform (Utilities|Array|Get(acopy) (Components|GetChildrenComponents (Variables|Default|GetSphere) false) _array_element) "None" "RTS_World")) "0, 0, 0" "0.050000,0.050000,0.050000") "Undefined" "OverrideRootScale" 0 (Variables|/Game/Cait/BP_SeedA.BP_SeedA_C|GetFlower%20Type _asbp_seed_a) self _array_element 0))
        (Utilities|Map|Add _slot _array_element true)
        (Utilities|Array|Add (Variables|Default|GetlistTunas) _returnvalue)
        (Default|SpawnNew _asbp_seed_a)
        (Actor|DestroyActor _asbp_seed_a)
        (goto _label Break)))))

(event EventBeginPlay)

(event Collision|EventActorBeginOverlap
  (params (OtherActor :type Actor%20Object%20Reference)))

(event EventTick
  (params (DeltaSeconds :type Float%20%28single-precision%29)))

(fn ConstructionScript)

(fn DeactivateSlot
  (params (slotNum :type Integer))
  (Utilities|Map|Add (Variables|Default|GetSlot) slotNum false))

(fn GrowPlant
  (for _array_element (Variables|Default|GetlistTunas)
    (Default|Grow _array_element))
  (Utilities|Array|Clear (Variables|Default|GetlistTunas)))