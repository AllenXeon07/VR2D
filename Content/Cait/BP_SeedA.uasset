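; Flower seed pickup actor that shows a paper sprite chosen by its FlowerType in the construction script.
; PickUpItem calls PickUp, which prints a message and destroys the actor after a short delay.
; SpawnNew and Respawn spawn a same-class copy at SpawnTransform with the same FlowerType, with Respawn also destroying the original.
; RotateToCamera yaws the sprite toward the player camera, while BeginPlay and Tick defer to the parent.
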(event Custom|SpawnNew
  (Game|SpawnActorfromClass (Utilities|GetClass self) (Variables|Default|GetSpawnTransform) "Undefined" "OverrideRootScale" 0 (Variables|Default|GetFlower%20Type) 0))

(event Custom|Destroy%20Item
  (Utilities|FlowControl|Delay 0.1)
  (Actor|DestroyActor))

(event Custom|Pick%20Up%20Item
  (CallFunction|PickUp))

(event EventBeginPlay
  (|CallParentFunction))

(event Collision|EventActorBeginOverlap
  (params (OtherActor :type Actor%20Object%20Reference)))

(event EventTick
  (params (DeltaSeconds :type Float%20%28single-precision%29))
  (|CallParentFunction DeltaSeconds))

(fn ConstructionScript
  (Rendering|Components|Sprite|SetSprite (Variables|Default|GetPaperSprite) (Utilities|Select :Index (- (Variables|Default|GetFlower%20Type) 1) :Option%200 "/Game/Cait/Asset/Flower1/Flower1Seed_Sprite.Flower1Seed_Sprite" :Option%201 "/Game/Cait/Asset/Flower2/Flower2Seed_Sprite.Flower2Seed_Sprite" :Option%202 "/Game/Cait/Asset/Flower3/Flower3Seed_Sprite.Flower3Seed_Sprite")))

(fn RotatetoCamera
  (bind _returnvalue (Transformation|GetActorLocation))
  (bind _returnvalue_2 (Game|GetPlayerCameraManager 0))
  (bind _returnvalue_3 (Transformation|GetActorLocation _returnvalue_2))
  (bind _returnvalue_4 (Math|Rotator|FindLookatRotation _returnvalue _returnvalue_3))
  (Transformation|SetWorldRotation (Variables|Default|GetPaperSprite) (Math|Rotator|MakeRotator 0.0 0.0 (+ (.yaw _returnvalue_4) 9e+01)) false false)
  (Transformation|SetWorldRotation (Variables|Default|GetPaperSprite) (Math|Rotator|MakeRotator 0.0 0.0 (.yaw _returnvalue_4)) false false))

(fn Respawn
  (bind _self self)
  (Game|SpawnActorfromClass (Utilities|GetClass _self) (Variables|Default|GetSpawnTransform) "Undefined" "OverrideRootScale" 0 (Variables|Default|GetFlower%20Type) 0)
  (Actor|DestroyActor _self))

(fn PickUp
  (Development|PrintString "Item Picked")
  (CallFunction|DestroyItem)
  (return 0))