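; BP_Flower1_Sprite is a billboarded flipbook sprite that stands in for a growing flower before being replaced by BP_Flower1.
; On BeginPlay, Grow sets the Flower1 flipbook, waits a fixed delay, then destroys the actor and spawns BP_Flower1 at the same transform.
; Each Tick, RotateToCamera turns the flipbook on yaw only to face the player camera, with a quarter-turn offset.
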(event Custom|Grow
  (Sprite|SetFlipbook (Variables|Default|GetPaperFlipbook) "/Game/Cait/Asset/2DSprite/Flower1_Flipbook.Flower1_Flipbook")
  (Utilities|FlowControl|Delay 9.5)
  (Actor|DestroyActor)
  (Game|SpawnActorfromClass "/Game/Cait/BP_Flower1.BP_Flower1_C" (Transformation|GetActorTransform) "Undefined" 0 0))

(event EventBeginPlay
  (CallFunction|Grow))

(event Collision|EventActorBeginOverlap
  (params (OtherActor :type Actor%20Object%20Reference)))

(event EventTick
  (params (DeltaSeconds :type Float%20%28single-precision%29))
  (CallFunction|RotatetoCamera))

(fn ConstructionScript)

(fn RotatetoCamera
  (Transformation|SetWorldRotation (Variables|Default|GetPaperFlipbook) (Math|Rotator|MakeRotator 0.0 0.0 (+ (.yaw (Math|Rotator|FindLookatRotation (Transformation|GetActorLocation) (Transformation|GetActorLocation (Game|GetPlayerCameraManager 0)))) 9e+01)) false false))