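; GM_Level, apparently the level's game mode, manages level streaming and keeps pot and seed counts.
; On BeginPlay it streams in the Map level, has BP_Store move the player, then streams in the Game level after a fixed delay.
; Tick counts TimeRemain down while Game is true and unloads the Game level only if the timer hits exactly zero.
; AddPot and AddSeed increment their counters.
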(event EventBeginPlay
  (Class|GameplayStatics|LoadStreamLevelbySoftObjectPtr "/Game/Map/Map.Map" true false)
  (bind _returnvalue (Actor|GetActorOfClass "/Game/Blueprint/BP_Store.BP_Store_C"))
  (bind _output_get (Variables|Default|SetStore _returnvalue))
  (Default|MovePlayer _output_get)
  (Utilities|FlowControl|Delay 1e+01)
  (Class|GameplayStatics|LoadStreamLevelbySoftObjectPtr "/Game/Map/Game.Game" true false))

(event EventTick
  (params (DeltaSeconds :type Float%20%28single-precision%29))
  (if (Variables|Default|GetGame)
    (bind _output_get (Variables|Default|SetTimeRemain (- (Variables|Default|GetTimeRemain) DeltaSeconds)))
    (if (== _output_get 0.0)
      (Class|GameplayStatics|UnloadStreamLevelbySoftObjectPtr "/Game/Map/Game.Game" false))))

(fn ConstructionScript)

(fn AddPot
  (bind _result (Math|Integer|IncrementInt (Variables|Default|GetPotCount))
    (:%20%20
      (Variables|Default|SetPotCount _result))))

(fn AddSeed
  (bind _result (Math|Integer|IncrementInt (Variables|Default|GetSeedCount))
    (:%20%20
      (Variables|Default|SetSeedCount _result))))