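; Base actor for a holdable tool object that returns to its starting place when left unheld.
; BeginPlay stores the spawn transform, and Tick runs a timer while Held is false; once it passes ReSpawnTime, Respawn spawns the same class at that transform and destroys this actor.
; ResetTime zeroes the timer and marks the object held, and ReleaseObject clears the flag.
; Action and DeAction are empty functions.
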(event EventBeginPlay
  (Variables|Default|SetSpawnTransform (Transformation|GetActorTransform)))

(event Collision|EventActorBeginOverlap
  (params (OtherActor :type Actor%20Object%20Reference)))

(event EventTick
  (params (DeltaSeconds :type Float%20%28single-precision%29))
  (if (not (Variables|Default|Getheld))
    (if (> (Variables|Default|GetcurrentTime) (Variables|Default|GetreSpawnTime))
      (CallFunction|Respawn)
      (else
        (Variables|Default|SetcurrentTime (+ (Variables|Default|GetcurrentTime) DeltaSeconds))))))

(fn ConstructionScript)

(fn Action)

(fn DeAction)

(fn ResetTime
  (Variables|Default|SetcurrentTime 0.0)
  (Variables|Default|Setheld true))

(fn Respawn
  (bind _self self)
  (bind _returnvalue (Game|SpawnActorfromClass (Utilities|GetClass _self) (Variables|Default|GetSpawnTransform) "Undefined" "MultiplyWithRoot" 0 0))
  (Actor|DestroyActor _self))

(fn ReleaseObject
  (Variables|Default|Setheld false))