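; Grabbable watering can that pours water when tilted and grows the BP_Pot plant beneath it.
; Each tick it compares the spout Arrow's dot product with world down against DotAngle to toggle the waterfall FX.
; While pouring, a downward line trace from the spout calls GrowPlant on any pot hit.
; CheckFar returns the physics Box to its spawn location and releases the grab when it strays too far.
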(event EventBeginPlay)

(event Collision|EventActorBeginOverlap
  (params (OtherActor :type Actor%20Object%20Reference)))

(event EventTick
  (params (DeltaSeconds :type Float%20%28single-precision%29))
  (bind _arrow (Variables|Default|GetArrow))
  (bind _fx_waterfall (Variables|Default|GetFX_Waterfall))
  (bind _returnvalue (Transformation|GetWorldLocation _arrow))
  (|CallParentFunction DeltaSeconds)
  (bind _outhit (Collision|LineTraceByChannel _returnvalue (+ _returnvalue "0.000000,0.000000,-1000.000000") "TraceTypeQuery1" false 0 "None" true "(R=1.000000,G=0.000000,B=0.000000,A=1.000000)" "(R=0.000000,G=1.000000,B=0.000000,A=1.000000)" 3.0))
  (Transformation|SetWorldLocation (Variables|Default|GetFX_Waterfall) _returnvalue false false)
  (if (< (Math|Vector|DotProduct (Math|Vector|GetForwardVector (Variables|Default|GetArrow)) "0.000000,0.000000,-1.000000") (Variables|Default|Getdot_angle))
    (Components|Activation|Activate _fx_waterfall false)
    (bind _asbp_pot (Utilities|Casting|CastToBP_Pot (.hitactor _outhit)))
    (Default|GrowPlant _asbp_pot)
    (else
      (Components|Activation|Deactivate _fx_waterfall))))

(fn ConstructionScript
  (Transformation|AttachComponentToComponent (Variables|Default|GetCube) 0 "None" "KeepRelative" "KeepRelative" "KeepRelative" true))

(fn CheckFar
  (bind _box (Variables|Default|GetBox))
  (if (> (Math|Vector|VectorLength (- (Transformation|GetWorldLocation _box) (Variables|Default|GetSpawnLocation))) 2e+02)
    (Physics|SetSimulatePhysics _box false)
    (Transformation|SetWorldLocation _box (Variables|Default|GetSpawnLocation) false false)
    (Physics|SetSimulatePhysics _box true)
    (Default|TryRelease (Variables|Default|GetGrabComponent))))