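; Level game mode for a plant shop game, running each timed round and tracking money, pot and seed type counts.
; Play loads the current level's limits and timer from a data table, resets counters and animates the sun via a timeline.
; Tick counts down while lerping sun rotation and color as a day cycle.
; After time expires and customers and NPCs are gone, it ends the round through BP_Store and clears pots and seeds.
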(event Custom|EndGame
  (Variables|Default|SetalreadyPlay false)
  (Class|GameplayStatics|UnloadStreamLevelbySoftObjectPtr "/Game/Map/Game.Game" false)
  (Default|EndGame (Variables|Default|GetStore))
  (bind _outactors (Actor|GetAllActorsOfClass "/Game/Cait/BP_Pot.BP_Pot_C"))
  (for _array_element _outactors
    (Actor|DestroyActor _array_element))
  (bind _outactors_2 (Actor|GetAllActorsOfClass "/Game/Cait/BP_Seed.BP_Seed_C"))
  (for _array_element_2 _outactors_2
    (Actor|DestroyActor _array_element_2)))

(event Custom|Reset
  (bind _datalevel (Variables|Default|GetDataLevel))
  (bind _sun (Variables|Default|GetSun))
  (bind _outrownames (DataTable|GetDataTableRowNames _datalevel))
  (Development|PrintString (Utilities|String|ToString(Name) (Utilities|Array|Get(acopy) _outrownames (- (Variables|Default|GetLevel) 1))))
  (bind _returnvalue (Utilities|GetDataTableRow _datalevel (Utilities|Array|Get(acopy) _outrownames (- (Variables|Default|GetLevel) 1)))
    (:then
      (Variables|Default|SetPotCount 0)
      (Variables|Default|SetSeedTypeCount 0)
      (Variables|Default|SetTimeRemain (.TimeRemain (Utilities|Struct|BreakS_Level _returnvalue)))
      (Variables|Default|SetMaxTypeCustomer (.MaxTypeCustomer (Utilities|Struct|BreakS_Level _returnvalue)))
      (Variables|Default|SetMaxSeedCount (.MaxSeedCount (Utilities|Struct|BreakS_Level _returnvalue)))
      (Variables|Default|SetMaxPotCount (.MaxPotCount (Utilities|Struct|BreakS_Level _returnvalue)))
      (Variables|Default|SetMaxFlowerCount (.MaxFlowerCount (Utilities|Struct|BreakS_Level _returnvalue)))
      (Variables|Default|SetMoney 7e+01)
      (Variables|Default|SetMaxTime (Variables|Default|GetTimeRemain))
      (bind _alpha (Timeline|ResetTimeline PlayFromStart)
        (:Update
          (Transformation|SetActorRotation _sun (Math|Rotator|MakeRotator -1.8e+02 (Math|Float|Lerp 359.0 181.0 _alpha) 1e+02))
          (Rendering|Components|Light|SetLightColor (Variables|/Script/Engine.Light|GetLightComponent _sun) (Math|Color|Lerp(LinearColor) "(R=0.784314,G=0.156863,B=0.536091,A=1.000000)" "(R=0.075000,G=0.443419,B=1.000000,A=1.000000)" _alpha) true))))))

(event Custom|play
  (Variables|Default|SetGame true)
  (Variables|Default|SetalreadyPlay true)
  (CallFunction|Reset))

(event EventBeginPlay
  (Class|GameplayStatics|LoadStreamLevelbySoftObjectPtr "/Game/Map/Map.Map" true false)
  (bind _returnvalue (Actor|GetActorOfClass "/Game/Blueprint/BP_Store.BP_Store_C"))
  (bind _output_get (Variables|Default|SetStore _returnvalue))
  (Default|MovePlayer _output_get)
  (Audio|PlaySound2D "/Game/Asset/Music/ES_Cheeky_Smiles.ES_Cheeky_Smiles" 1.0 1.0 0.0 0 0)
  (bind _returnvalue_2 (Actor|GetActorOfClass "/Script/Engine.DirectionalLight"))
  (Variables|Default|SetSun _returnvalue_2))

(event EventTick
  (params (DeltaSeconds :type Float%20%28single-precision%29))
  (bind _sun (Variables|Default|GetSun))
  (if (Variables|Default|GetGame)
    (bind _output_get (Variables|Default|SetTimeRemain (Math|Float|Max(Float) (- (Variables|Default|GetTimeRemain) DeltaSeconds) 0.0)))
    (Transformation|SetActorRotation _sun (Math|Rotator|MakeRotator -1.8e+02 (Math|Float|Lerp 359.0 181.0 (/ _output_get (Variables|Default|GetMaxTime))) 1e+02))
    (Rendering|Components|Light|SetLightColor (Variables|/Script/Engine.Light|GetLightComponent _sun) (Math|Color|Lerp(LinearColor) "(R=0.784314,G=0.156863,B=0.536091,A=1.000000)" "(R=0.075000,G=0.443419,B=1.000000,A=1.000000)" (/ _output_get (Variables|Default|GetMaxTime))) true)
    (if (<= _output_get 0.0)
      (Variables|Default|SetGame false))
    (elif (Variables|Default|GetalreadyPlay)
      (bind _outactors (Actor|GetAllActorsOfClass "/Game/Blueprint/NPC/BP_Customer.BP_Customer_C"))
      (bind _outactors_2 (Actor|GetAllActorsOfClass "/Game/Blueprint/NPC/BP_NPC.BP_NPC_C"))
      (if (== (+ (Utilities|Array|Length _outactors_2) (Utilities|Array|Length _outactors)) 0)
        (CallFunction|EndGame)))))

(fn ConstructionScript)

(fn AddPot
  (bind _result (Math|Integer|IncrementInt (Variables|Default|GetPotCount))
    (:%20%20
      (Variables|Default|SetPotCount _result))))

(fn AddSeed
  (bind _result (Math|Integer|IncrementInt (Variables|Default|GetSeedTypeCount))
    (:%20%20
      (Variables|Default|SetSeedTypeCount _result))))

(fn AddMoney
  (params (income :type Float%20%28double-precision%29))
  (Variables|Default|SetMoney (+ (Variables|Default|GetMoney) income)))