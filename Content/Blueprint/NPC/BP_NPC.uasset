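; BP_NPC is a flipbook sprite NPC that walks along a referenced Path spline and destroys itself at the end.
; Construction assigns the source flipbook, and Tick yaws the sprite to face the player camera as a billboard.
; The Moving event chains AI MoveTo calls to successive spline points, stepping a normalized distance forward after each move, whether it succeeds or fails.
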(event Custom|Moving
  (bind _path (Variables|Default|GetPath))
  (bind _spline (Variables|/Game/Blueprint/NPC/BP_Path.BP_Path_C|GetSpline _path))
  (AI|AIMoveTo self (Spline|GetLocationatDistanceAlongSpline _spline (Math|Float|Lerp 0.0 (Spline|GetSplineLength _spline) (Variables|Default|Getdistance)) "World") 0 5.0 false :!label _label
    (:OnSuccess
      _)
    (:OnFail
      _))
  (bind _output_get (Variables|Default|Setdistance (+ (Variables|Default|Getdistance) 0.005)))
  (if (> _output_get 1.0)
    (Actor|DestroyActor)
    (else
      (goto _label))))

(event EventBeginPlay)

(event Collision|EventActorBeginOverlap
  (params (OtherActor :type Actor%20Object%20Reference)))

(event EventTick
  (params (DeltaSeconds :type Float%20%28single-precision%29))
  (CallFunction|RotatetoCamera))

(fn ConstructionScript
  (Sprite|SetFlipbook (Variables|Default|GetSprite) (Variables|Default|GetSourceFlipbook)))

(fn RotatetoCamera
  (Transformation|SetWorldRotation (Variables|Default|GetSprite) (Math|Rotator|MakeRotator 0.0 0.0 (+ (.yaw (Math|Rotator|FindLookatRotation (Transformation|GetActorLocation) (Transformation|GetActorLocation (Game|GetPlayerCameraManager 0)))) 9e+01)) false false))