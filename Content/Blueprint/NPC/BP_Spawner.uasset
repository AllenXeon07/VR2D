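; Customer spawner that keeps a counter staffed with a customer while the level's game mode reports the game running.
; On a configurable tick interval, it checks whether the counter is free and spawns a normal, angry or special customer.
; Power and log math expressions skew the random type choice, bounded by the game mode's MaxTypeCustomer.
; The new customer is sent to the counter with a leave location and registered as its occupant.
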(event EventTick
  (params (DeltaSeconds :type Float%20%28single-precision%29))
  (bind _returnvalue (|(pow(10,(1/x))) 1.0))
  (bind _gm (Variables|Default|GetGM))
  (bind _returnvalue_2 (Math|Float|Round _returnvalue))
  (bind _maxtypecustomer (Variables|/Game/Blueprint/GM_Level.GM_Level_C|GetMaxTypeCustomer _gm))
  (bind _returnvalue_3 (+ _maxtypecustomer 1))
  (bind _returnvalue_4 (Math|Conversions|ToFloat(Integer) _returnvalue_3))
  (bind _returnvalue_5 (|(pow(10,(1/x))) _returnvalue_4))
  (bind _returnvalue_6 (+ _returnvalue_5 1.0))
  (bind _returnvalue_7 (Math|Random|RandomIntegerinRange _returnvalue_6 _returnvalue_2))
  (if (Variables|/Game/Blueprint/GM_Level.GM_Level_C|GetGame (Variables|Default|GetGM))
    (Utilities|IsValid (Variables|/Game/Blueprint/NPC/BP_SlotCounter.BP_SlotCounter_C|GetCustomer (Variables|Default|GetCounter%20Location))
      (:Is%20Not%20Valid
        (Development|PrintString (Utilities|String|ToString(Integer) _returnvalue_7))
        (bind _returnvalue_8 (Game|SpawnActorfromClass (Utilities|Select :Index (- (Math|Float|Round (|(1/(log(x,10))) (Math|Conversions|ToFloat(Integer) _returnvalue_7))) 1) :Option%200 "/Game/Blueprint/NPC/BP_CNormal.BP_CNormal_C" :Option%201 "/Game/Blueprint/NPC/BP_CAngry.BP_CAngry_C" :Option%202 "/Game/Blueprint/NPC/BP_CSpecial.BP_CSpecial_C") (Transformation|GetActorTransform) "AdjustIfPossibleButAlwaysSpawn" "MultiplyWithRoot" 0 0))
        (bind _asbp_customer (Utilities|Casting|CastToBP_Customer _returnvalue_8))
        (Default|GottoCounter _asbp_customer (Variables|Default|GetCounter%20Location) (Variables|Default|GetLeave%20Location))
        (Variables|/Game/Blueprint/NPC/BP_SlotCounter.BP_SlotCounter_C|SetCustomer (Variables|Default|GetCounter%20Location) _asbp_customer)))))

(event EventBeginPlay
  (Actor|Tick|SetActorTickInterval (Variables|Default|GetTick%20Interval))
  (bind _asgm_level (Utilities|Casting|CastToGM_Level (Game|GetGameMode)))
  (Variables|Default|SetGM _asgm_level))

(fn ConstructionScript)