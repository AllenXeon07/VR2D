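; BP_SlotCounter is a counter slot actor where a bucket is handed over to a customer.
; Its Box overlap stores an entering BP_Bucket and calls GiveBucket, while end overlap clears the reference.
; If available, GiveBucket waits briefly, asks the Customer to check the bucket, and on a match makes the customer leave and destroys the bucket.
; SetAvailable toggles the slot and shows or hides its Cube in game.
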(event OnComponentBeginOverlap(Box)
  (params (OverlappedComponent :type Primitive%20Component%20Object%20Reference) (OtherActor :type Actor%20Object%20Reference) (OtherComp :type Primitive%20Component%20Object%20Reference) (OtherBodyIndex :type Integer) (bFromSweep :type Boolean) (SweepResult :type Hit%20Result%20Structure%20%28by%20ref%29))
  (bind _asbp_bucket (Utilities|Casting|CastToBP_Bucket OtherActor))
  (Variables|Default|SetBucket _asbp_bucket)
  (CallFunction|GiveBucket)
  (Development|PrintString (Utilities|GetDisplayName OtherActor)))

(event OnComponentEndOverlap(Box)
  (params (OverlappedComponent :type Primitive%20Component%20Object%20Reference) (OtherActor :type Actor%20Object%20Reference) (OtherComp :type Primitive%20Component%20Object%20Reference) (OtherBodyIndex :type Integer))
  (Utilities|Casting|CastToBP_Bucket OtherActor)
  (Variables|Default|SetBucket 0))

(event Custom|GiveBucket
  (bind _customer (Variables|Default|GetCustomer))
  (bind _bucket (Variables|Default|GetBucket))
  (if (Variables|Default|Getavailable)
    (Utilities|FlowControl|Delay 1.0)
    (Utilities|IsValid _bucket
      (:Is%20Valid
        (Utilities|IsValid _customer
          (:Is%20Valid
            (bind _correctbucket (Default|CheckBucket _customer _bucket))
            (if _correctbucket
              (Default|Leave _customer)
              (Actor|DestroyActor _bucket)
              (Development|PrintString "Correct"))))))))

(event EventBeginPlay
  (|CallParentFunction) ; This node is disabled and will not be called.\nDrag off pins to build functionality.
)

(event Collision|EventActorBeginOverlap
  (params (OtherActor :type Actor%20Object%20Reference))
  (|CallParentFunction OtherActor) ; This node is disabled and will not be called.\nDrag off pins to build functionality.
)

(event EventTick
  (params (DeltaSeconds :type Float%20%28single-precision%29))
  (|CallParentFunction DeltaSeconds))

(fn ConstructionScript
  (|CallParentFunction))

(fn SetAvailable
  (params (available :type Boolean))
  (bind _output_get (Variables|Default|Setavailable available))
  (Development|SetHiddeninGame (Variables|Default|GetCube) (not _output_get) false))