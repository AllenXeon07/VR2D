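; BP_CTestNormal is an NPC Blueprint, apparently a test variant, that displays a flower seed order in a widget.
; On BeginPlay it loops over a one-element array and picks one of three flower seed images, indexed by RandomSelect minus the element.
; It creates a WB_FlowerIcon with that image and adds it to the container of the WB_Order held by its Widget component.
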(event EventBeginPlay
  (for _array_element (Utilities|Array|MakeArray 0)
    (bind _aswb_order (Utilities|Casting|CastToWB_Order (UserInterface|GetWidget (Variables|Default|GetWidget))))
    (bind _returnvalue (UserInterface|CreateWidget "/Game/Blueprint/NPC/WB_FlowerIcon.WB_FlowerIcon_C" 0 (Utilities|Select :Index (- (Variables|Default|GetRandomSelect) _array_element) :Option%200 "/Game/Asset/2D/Seed/Flower1Seed.Flower1Seed" :Option%201 "/Game/Asset/2D/Seed/Flower2Seed.Flower2Seed" :Option%202 "/Game/Asset/2D/Seed/Flower3Seed.Flower3Seed")))
    (Default|AddtoContainer _aswb_order _returnvalue)))

(event Collision|EventActorBeginOverlap
  (params (OtherActor :type Actor%20Object%20Reference))
  (|CallParentFunction OtherActor) ; This node is disabled and will not be called.\nDrag off pins to build functionality.
)

(event EventTick
  (params (DeltaSeconds :type Float%20%28single-precision%29))
  (|CallParentFunction DeltaSeconds) ; This node is disabled and will not be called.\nDrag off pins to build functionality.
)

(fn ConstructionScript)