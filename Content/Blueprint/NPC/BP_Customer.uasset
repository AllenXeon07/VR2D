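; Flower shop customer NPC that rolls a random flower order from game mode limits and shows it as icons in a widget.
; It AI-moves to a counter, requests a bucket and waits as the order reddens, calling an empty Angry hook and leaving on timeout.
; Tick yaw-billboards the sprite and widget toward the camera.
; CheckBucket compares flower counts against the order; Pay adds per-flower prices plus a flat bonus to game mode money.
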(event Custom|Leave
  (Rendering|SetVisibility (Variables|Default|GetWidget) false false)
  (Variables|Default|Setleaving true)
  (Default|SetAvailable (Variables|Default|GetCounterLocation) false)
  (AI|AIMoveTo self (+ (Transformation|GetActorLocation) "0.000000,100.000000,0.000000") 0 5.0 false
    (:OnSuccess
      _)
    (:OnFail
      _))
  (AI|AIMoveTo self "0, 0, 0" (Variables|Default|GetLeaveLocation) 5.0 false
    (:OnSuccess
      (Actor|DestroyActor))))

(event Custom|GotToCounter
  (params (CounterLocation :type BP%20Slot%20Counter%20Object%20Reference) (LeaveLocation :type Actor%20Object%20Reference))
  (Variables|Default|SetCounterLocation CounterLocation)
  (Variables|Default|SetLeaveLocation LeaveLocation)
  (AI|AIMoveTo self "0, 0, 0" (Variables|Default|GetCounterLocation) 5.0 false
    (:OnSuccess
      (Variables|Default|Setwaiting true)
      (Rendering|SetVisibility (Variables|Default|GetWidget) true true)
      (Rendering|SetVisibility (Variables|Default|GetWidget) true false)
      (Default|SetAvailable (Variables|Default|GetCounterLocation) true)
      (Default|GiveBucket (Variables|Default|GetCounterLocation))
      (Utilities|FlowControl|Delay (Variables|Default|GetWait))
      (if (not (Variables|Default|Getleaving))
        (CallFunction|Angry)
        (CallFunction|Leave)
        (Variables|/Game/Blueprint/NPC/BP_SlotCounter.BP_SlotCounter_C|SetCustomer (Variables|Default|GetCounterLocation) 0)))))

(event Custom|Angry)

(event EventBeginPlay
  (bind _orderlist (Variables|Default|GetOrderList))
  (bind _asgm_level (Utilities|Casting|CastToGM_Level (Game|GetGameMode)))
  (bind _output_get (Variables|Default|SetFlowerCount (Math|Random|RandomIntegerinRange 1 (Variables|/Game/Blueprint/GM_Level.GM_Level_C|GetMaxFlowerCount _asgm_level))))
  (for _index (range 1 _output_get)
    (bind _output_get_2 (Variables|Default|SetRandomSelect (Math|Random|RandomIntegerinRange 1 (Variables|/Game/Blueprint/GM_Level.GM_Level_C|GetMaxSeedCount _asgm_level))))
    (bind _result (Math|Integer|IncrementInt (.Value (Utilities|Map|Find _orderlist _output_get_2)))
      (:%20%20
        (Utilities|Map|Add _orderlist _output_get_2 _result)
        (bind _aswb_order (Utilities|Casting|CastToWB_Order (UserInterface|GetWidget (Variables|Default|GetWidget))))
        (bind _returnvalue (UserInterface|CreateWidget "/Game/Blueprint/NPC/WB_FlowerIcon.WB_FlowerIcon_C" 0 (Utilities|Select :Index (- (Variables|Default|GetRandomSelect) 1) :Option%200 "/Game/Asset/2D/Flower/Icon1.Icon1" :Option%201 "/Game/Asset/2D/Flower/Icon2.Icon2" :Option%202 "/Game/Asset/2D/Flower/Icon3.Icon3")))
        (Default|AddtoContainer _aswb_order _returnvalue)))))

(event EventTick
  (params (DeltaSeconds :type Float%20%28single-precision%29))
  (CallFunction|RotatetoCamera)
  (if (Variables|Default|Getwaiting)
    (Variables|Default|SetcurrentTime (+ (Variables|Default|GetcurrentTime) DeltaSeconds))
    (bind _aswb_order (Utilities|Casting|CastToWB_Order (UserInterface|GetWidget (Variables|Default|GetWidget))))
    (Default|SetColor _aswb_order (Utilities|Struct|MakeSlateColor (Math|Color|Lerp(LinearColor) "(R=0.141176,G=0.141176,B=0.141176,A=1.000000)" "(R=0.141176,G=0.016912,B=0.016912,A=1.000000)" (/ (Variables|Default|GetcurrentTime) (Variables|Default|GetWait))) "UseColor_Specified"))))

(fn ConstructionScript)

(fn RotatetoCamera
  (bind _returnvalue (Game|GetPlayerCameraManager 0))
  (bind _returnvalue_2 (Transformation|GetActorLocation))
  (bind _returnvalue_3 (Transformation|GetActorLocation _returnvalue))
  (bind _returnvalue_4 (Math|Rotator|FindLookatRotation _returnvalue_2 _returnvalue_3))
  (Transformation|SetWorldRotation (Variables|Default|GetSprite) (Math|Rotator|MakeRotator 0.0 0.0 (+ (.yaw _returnvalue_4) 9e+01)) false false)
  (Transformation|SetWorldRotation (Variables|Default|GetWidget) (Math|Rotator|MakeRotator 0.0 0.0 (.yaw _returnvalue_4)) false false))

(fn CheckBucket
  (params (Bucket :type BP%20Bucket%20Object%20Reference))
  (bind _orderlist (Variables|Default|GetOrderList))
  (bind _keys (Utilities|Map|Keys _orderlist))
  (bind _array_element (Utilities|Array|ForEachLoopwithBreak _keys)
    (:LoopBody
      (if (not (== (.Value (Utilities|Map|Find _orderlist _array_element)) (.Value (Utilities|Map|Find (Variables|/Game/Blueprint/Flower/BP_Bucket.BP_Bucket_C|GetFlowerList Bucket) _array_element))))
        (return false)))
    (:Completed
      (return true))))

(fn Pay
  (params (Bouquet :type BP%20Bucket%20Object%20Reference))
  (bind _flowerlist (Variables|/Game/Blueprint/Flower/BP_Bucket.BP_Bucket_C|GetFlowerList Bouquet))
  (bind _asgm_level (Utilities|Casting|CastToGM_Level (Game|GetGameMode)))
  (LocalVariables|SetGM _asgm_level)
  (LocalVariables|SetTotalPayment 0.0)
  (bind _keys (Utilities|Map|Keys _flowerlist))
  (for _array_element _keys
    (LocalVariables|SetTotalPayment (+ (LocalVariables|GetTotalPayment) (* (.Value (Utilities|Map|Find _flowerlist _array_element)) (.Value (Utilities|Map|Find (Variables|/Game/Blueprint/GM_Level.GM_Level_C|GetFlowerSoldPrice (LocalVariables|GetGM)) _array_element))))))
  (Default|AddMoney (LocalVariables|GetGM) (+ (LocalVariables|GetTotalPayment) 1e+01)))