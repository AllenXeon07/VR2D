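; BP_Flower3D is a placeable 3D flower actor that can be cut to produce a pickup.
; Its construction script picks one of three flower meshes from the one-based FlowerType and scales it down uniformly.
; The Cut event spawns a BP_FlowerPick at the flower's location with the same FlowerType, then destroys the flower.
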(event Custom|Cut
  (Game|SpawnActorfromClass "/Game/Blueprint/Flower/BP_FlowerPick.BP_FlowerPick_C" (Math|Conversions|ToTransform(Vector) (Transformation|GetActorLocation)) "Undefined" "MultiplyWithRoot" 0 (Variables|Default|GetflowerType) 0)
  (Actor|DestroyActor))

(event EventBeginPlay)

(event Collision|EventActorBeginOverlap
  (params (OtherActor :type Actor%20Object%20Reference)))

(event EventTick
  (params (DeltaSeconds :type Float%20%28single-precision%29)))

(fn ConstructionScript
  (bind _staticmesh (Variables|Default|GetStaticMesh))
  (Components|StaticMesh|SetStaticMesh _staticmesh (Utilities|Select :Index (- (Variables|Default|GetflowerType) 1) :Option%200 "/Game/Asset/3D/Flower1/Flower1_3DModel.Flower1_3DModel" :Option%201 "/Game/Asset/3D/Flower2/Flower2_3DModel.Flower2_3DModel" :Option%202 "/Game/Asset/3D/Flower3/Flower3_3DModel.Flower3_3DModel"))
  (Transformation|SetWorldScale3D _staticmesh "0.050000,0.050000,0.050000"))