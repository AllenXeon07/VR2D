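; BP_Bucket is a flower bucket that collects up to three picked flowers.
; When a BP_FlowerPick overlaps its Box, the next of three mesh slots gets the flower-on-stick mesh matching that flower's type.
; It then increments a per-type tally in the FlowerList map, kept for comparison, and destroys the picked flower.
; Despite its name, Respawn only destroys the bucket.
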(event OnComponentBeginOverlap(Box)
  (params (OverlappedComponent :type Primitive%20Component%20Object%20Reference) (OtherActor :type Actor%20Object%20Reference) (OtherComp :type Primitive%20Component%20Object%20Reference) (OtherBodyIndex :type Integer) (bFromSweep :type Boolean) (SweepResult :type Hit%20Result%20Structure%20%28by%20ref%29))
  (bind _flowerlist (Variables|Default|GetFlowerList))
  (if (< (Variables|Default|GetFlowerCount) 3)
    (bind _asbp_flower_pick (Utilities|Casting|CastToBP_FlowerPick OtherActor))
    (Components|StaticMesh|SetStaticMesh (Utilities|Array|Get(acopy) (Variables|Default|GetFlowerMesh) (Variables|Default|GetFlowerCount)) (Utilities|Select :Index (- (Variables|/Game/Blueprint/Flower/BP_FlowerPick.BP_FlowerPick_C|GetflowerType _asbp_flower_pick) 1) :Option%200 "/Game/Asset/3D/Flower1/Flowernstick1.Flowernstick1" :Option%201 "/Game/Asset/3D/Flower2/Flowernstick2.Flowernstick2" :Option%202 "/Game/Asset/3D/Flower3/Flowernstick3.Flowernstick3"))
    (bind _result (Math|Integer|IncrementInt (Variables|Default|GetFlowerCount))
      (:%20%20
        (Variables|Default|SetFlowerCount _result)
        ;[1 1 1] Set To FlowerList for Comparison
        (Utilities|Map|Add _flowerlist (Variables|/Game/Blueprint/Flower/BP_FlowerPick.BP_FlowerPick_C|GetflowerType _asbp_flower_pick) (+ (.Value (Utilities|Map|Find _flowerlist (Variables|/Game/Blueprint/Flower/BP_FlowerPick.BP_FlowerPick_C|GetflowerType _asbp_flower_pick))) 1))
        (Actor|DestroyActor _asbp_flower_pick)))))

(event EventBeginPlay
  (|CallParentFunction)
  (Variables|Default|SetFlowerMesh (Utilities|Array|MakeArray (Variables|Default|GetFlower1) (Variables|Default|GetFlower2) (Variables|Default|GetFlower3))))

(event Collision|EventActorBeginOverlap
  (params (OtherActor :type Actor%20Object%20Reference))
  (|CallParentFunction OtherActor) ; This node is disabled and will not be called.\nDrag off pins to build functionality.
)

(event EventTick
  (params (DeltaSeconds :type Float%20%28single-precision%29))
  (|CallParentFunction DeltaSeconds) ; This node is disabled and will not be called.\nDrag off pins to build functionality.
)

(fn ConstructionScript)

(fn Respawn
  (Actor|DestroyActor))