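; BP_FlowerPick is a flower prop actor, apparently for picking, that displays one of three flower-on-stick meshes.
; Its construction script uses the FlowerType variable, offset by one, to select the static mesh and then shrinks it to a small uniform world scale.
; The event graph holds only disabled default events, so this Blueprint contains no pickup or runtime logic of its own.
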(event EventBeginPlay
  (|CallParentFunction) ; This node is disabled and will not be called.\nDrag off pins to build functionality.
)

(event Collision|EventActorBeginOverlap
  (params (OtherActor :type Actor%20Object%20Reference))
  (|CallParentFunction OtherActor) ; This node is disabled and will not be called.\nDrag off pins to build functionality.
)

(event EventTick
  (params (DeltaSeconds :type Float%20%28single-precision%29))
  (|CallParentFunction DeltaSeconds) ; This node is disabled and will not be called.\nDrag off pins to build functionality.
)

(fn ConstructionScript
  (bind _staticmesh (Variables|Default|GetStaticMesh))
  (|CallParentFunction)
  (Components|StaticMesh|SetStaticMesh _staticmesh (Utilities|Select :Index (- (Variables|Default|GetflowerType) 1) :Option%200 "/Game/Asset/3D/Flower1/Flowernstick1.Flowernstick1" :Option%201 "/Game/Asset/3D/Flower2/Flowernstick2.Flowernstick2" :Option%202 "/Game/Asset/3D/Flower3/Flowernstick3.Flowernstick3"))
  (Transformation|SetWorldScale3D _staticmesh "0.050000,0.050000,0.050000"))