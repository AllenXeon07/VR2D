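; Blueprint function library with a helper that counts seeds of a given flower type in the level.
; CountSeed gathers every BP_Seed actor through GetAllActorsOfClass and loops over them.
; It increments a local counter for each seed whose FlowerType matches the requested type and returns the total.
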(fn CountSeed
  (params (type :type Integer))
  (LocalVariables|SetSeedCount 0)
  (bind _outactors (Actor|GetAllActorsOfClass 0 "/Game/Cait/BP_Seed.BP_Seed_C"))
  (for _array_element _outactors
    (if (== (Variables|/Game/Cait/BP_Seed.BP_Seed_C|GetFlower%20Type _array_element) type)
      (Math|Integer|IncrementInt (LocalVariables|GetSeedCount)
        (:%20%20
          (LocalVariables|SetSeedCount (LocalVariables|GetSeedCount))))))
  (return (LocalVariables|GetSeedCount)))